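; DangerBee game mode that tracks flower-bloom progress, shows it in a counter widget and feeds it to the music.
; UpdateWB scans all BP_Flower actors, locks the unbloomed total on first run and increments the bloomed count on every call, including BeginPlay's.
; Tick sends the resulting percentage to the music's "Flowers" parameter.
; A short BeginPlay timer fires the end-game event, whose bound handler only prints a message.
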(event Custom|UpdateWB
  (Utilities|FlowControl|Sequence
    (:then_0
      (bind _outactors (Actor|GetAllActorsOfClass "/Game/Blueprints/BP_Flower.BP_Flower_C"))
      (for _array_element _outactors
        (if (Variables|/Game/Blueprints/BP_Flower.BP_Flower_C|Getis_Bloomed _array_element)
          (Math|Integer|IncrementInt (Variables|Default|GetBloomyCount)
            (:%20%20
              (Rendering|SetVisibility (Variables|/Game/Blueprints/BP_Flower.BP_Flower_C|GetMaterialBillboard _array_element) false false)))
          (else
            (Math|Integer|IncrementInt (Variables|Default|GetNotBloomedCounter))))))
    (:then_1
      (if (not (Variables|Default|GetFirstCheck))
        (Variables|Default|SetTotalUnBloomed (Variables|Default|GetNotBloomedCounter))
        (Variables|Default|SetFirstCheck true)))
    (:then_2
      (Math|Integer|IncrementInt (Variables|Default|GetNewlyBloomed)))
    (:then_3
      (Variables|Default|SetPercentage (/ (Math|Conversions|ToFloat(Integer) (Variables|Default|GetNewlyBloomed)) (Math|Conversions|ToFloat(Integer) (Variables|Default|GetTotalUnBloomed))))
      (Variables|Default|SetBloomyCount 0)
      (Variables|/Game/Blueprints/UI/UI_BloomCounter.UI_BloomCounter_C|SetRemaining (Variables|Default|GetUI_BloomCounter) (Utilities|Text|ToText(String) (Utilities|String|Append (Utilities|String|ToString(Integer) (Variables|Default|GetNewlyBloomed)) "/" (Utilities|String|ToString(Integer) (Variables|Default|GetTotalUnBloomed)))))
      (Variables|Default|SetNotBloomedCounter 0))))

(event Custom|End
  (Development|PrintString "end game trigger" true true "(R=0.000000,G=0.660000,B=1.000000,A=1.000000)" 2e+01))

(event EventBeginPlay
  (bind _returnvalue (UserInterface|CreateWidget "/Game/Blueprints/UI/UI_BloomCounter.UI_BloomCounter_C"))
  (bind _output_get (Variables|Default|SetUI_BloomCounter _returnvalue))
  (UserInterface|Viewport|AddtoViewport _output_get 0)
  (CallFunction|UpdateWB)
  (bind _returnvalue_2 (Utilities|Time|SetTimerbyFunctionName self "CountDown" 5.0))
  (Utilities|Time|UnpauseTimerbyHandle _returnvalue_2)
  (EventDispatchers|BindEventtoEndGame (delegate Custom|End)))

(event EventTick
  (params (DeltaSeconds :type Float%20%28single-precision%29))
  (Class|FMODAudioComponent|SetParameter (Variables|Default|GetMusic) "Flowers" (* (Variables|Default|GetPercentage) 1e+02)))

(fn ConstructionScript)

(fn UpdateCounter
  (bind _result (Math|Integer|IncrementInt (Variables|Default|GetCounter))
    (:%20%20
      (return _result))))

(fn UpdateBloomCount
  (params (Index :type Integer) (BLooming? :type Boolean))
  (bind _bloomornah_ (Variables|Default|GetBloomOrNah?))
  (Utilities|Array|Resize _bloomornah_ Index)
  (Utilities|Array|Insert _bloomornah_ BLooming? Index))

(fn CountDown
  (Default|CallEndGame))