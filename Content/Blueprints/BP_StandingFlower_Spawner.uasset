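; Standing flower spawner that blooms into peppers or tomatoes when an actor with "Bee" in its name overlaps its capsule.
; The first overlap sets IsBloomed, shows the billboard and a produce component, spawns pollen particles at the stick and plays Bloom.
; Produce gets random scale and red or green tint through a dynamic material.
; RandomBool picks separately per step, so shown, tinted and scaled components can differ.
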(event OnComponentBeginOverlap(Capsule)
  (params (OverlappedComponent :type Primitive%20Component%20Object%20Reference) (OtherActor :type Actor%20Object%20Reference) (OtherComp :type Primitive%20Component%20Object%20Reference) (OtherBodyIndex :type Integer) (bFromSweep :type Boolean) (SweepResult :type Hit%20Result%20Structure%20%28by%20ref%29))
  (bind _returnvalue (Math|Random|RandomBool))
  (bind _returnvalue_2 (Math|Random|RandomFloatinRange 0.7 1.2))
  (bind _materialbillboard (Variables|Default|GetMaterialBillboard))
  (bind _peppers (Variables|Default|GetPeppers))
  (bind _standingstick (Variables|Default|GetStandingStick))
  (bind _tomatos (Variables|Default|GetTomatos))
  (bind _returnvalue_3 (Transformation|GetWorldTransform _standingstick))
  (bind _returnvalue_4 (select _returnvalue _peppers _tomatos))
  (if (Utilities|String|Contains (Utilities|GetObjectName OtherActor) "Bee")
    (if (Variables|Default|GetIsBloomed)
      (Rendering|SetVisibility _materialbillboard (stale _output_get) false)
      (else
        (bind _output_get (Variables|Default|SetIsBloomed true))
        (Rendering|SetVisibility _materialbillboard _output_get false)
        (Rendering|SetVisibility _returnvalue_4 true false)
        (bind _returnvalue_5 (Rendering|Material|CreateDynamicMaterialInstance _returnvalue_4 0 (Rendering|Material|GetMaterial _returnvalue_4 0) :!class /Script/Engine.PrimitiveComponent))
        (Transformation|SetRelativeScale3D _returnvalue_4 (Math|Vector|MakeVector _returnvalue_2 _returnvalue_2 _returnvalue_2))
        (bind _output_get_2 (Variables|Default|SetFlowerHeadColour (Math|Color|SelectColor "(R=1.000000,G=0.015526,B=0.000000,A=1.000000)" "(R=0.146672,G=0.828125,B=0.038818,A=1.000000)" (Math|Random|RandomBool))))
        (Rendering|Material|SetVectorParameterValue _returnvalue_5 "BC | Colour Adjustment 1" _output_get_2 :!class /Script/Engine.MaterialInstanceDynamic)
        (Rendering|Material|SetVectorParameterValue _returnvalue_5 "BC | Colour Adjustment 2" _output_get_2 :!class /Script/Engine.MaterialInstanceDynamic)
        (Effects|SpawnEmitteratLocation "/Game/Assets/ParticleSystems/pollen_particles.pollen_particles" (.location _returnvalue_3) (.rotation _returnvalue_3) (* (.scale _returnvalue_3) "1.500000,1.500000,1.500000"))
        (Class|FMODAudioComponent|Play (Variables|Default|GetBloom))))))

(fn ConstructionScript)