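; Snail pawn that wanders the NavMesh on a looping timer, squeaking at random.
; Overlap with either bee type stops it, pauses wandering, hides its body and plays a scream; after separation, a polling timer restores it with a bop sound.
; Flower seeking and climbing, animated by self-registering looping timers, is present but dormant: its entry points are unwired or never called from the live wander logic.
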(event OnComponentBeginOverlap(CapsuleComponent)
  (params (OverlappedComponent :type Primitive%20Component%20Object%20Reference) (OtherActor :type Actor%20Object%20Reference) (OtherComp :type Primitive%20Component%20Object%20Reference) (OtherBodyIndex :type Integer) (bFromSweep :type Boolean) (SweepResult :type Hit%20Result%20Structure%20%28by%20ref%29))
  (Utilities|Casting|CastToBP_Bee_Redo OtherActor
    (:then
      _)
    (:CastFailed
      (Utilities|Casting|CastToBP_Flying_Bee OtherActor)))
  (CallFunction|OnBeeOverlap))

(event OnComponentEndOverlap(CapsuleComponent)
  (params (OverlappedComponent :type Primitive%20Component%20Object%20Reference) (OtherActor :type Actor%20Object%20Reference) (OtherComp :type Primitive%20Component%20Object%20Reference) (OtherBodyIndex :type Integer))
  (Utilities|Casting|CastToBP_Bee_Redo OtherActor
    (:then
      _)
    (:CastFailed
      (Utilities|Casting|CastToBP_Flying_Bee OtherActor)))
  (CallFunction|OnBeeEndOverlap))

(event Custom|SearchForFlower
  (CallFunction|GetNewFlower)
  (CallFunction|MovetoFlower))

(event EventBeginPlay
  (CallFunction|InitSnailStuff)
  (bind _returnvalue (Utilities|Time|SetTimerbyFunctionName self "Wander" (Math|Random|RandomFloatinRange 2.0 3.5) true))
  (Utilities|Time|UnpauseTimerbyHandle _returnvalue)
  (CallFunction|Wander))

(event EventTick
  (params (DeltaSeconds :type Float%20%28single-precision%29))
  (if (== (Math|Random|RandomInteger 300) 234)
    (Class|FMODAudioComponent|Play (Variables|Default|GetSquick))))

(fn ConstructionScript)

(fn MovetoFlower
  (bind _asaic_snail_aicontroller (Utilities|Casting|CastToAIC_SnailAIController (AI|GetAIController self)))
  (Pawn|Components|CharacterMovement|SetMovementMode (Variables|Character|GetCharacterMovement) "MOVE_Walking" 0)
  (AI|Navigation|MovetoActor _asaic_snail_aicontroller (Variables|Default|GetFlowerTarget) 5.0 false true))

(fn InitSnailStuff
  (Variables|/Script/Engine.CharacterMovementComponent|SetMaxWalkSpeed (Variables|Character|GetCharacterMovement) (Variables|Default|GetMoveSpeed)))

(fn ClimbFlower
  (bind _returnvalue (Utilities|String|MakeLiteralString "ClimbFlower"))
  (bind _returnvalue_2 (Transformation|GetActorRotation))
  (bind _self self)
  (if (Class|KismetSystemLibrary|TimerExists _self _returnvalue)
    (Transformation|SetActorRotation (Math|Rotator|MakeRotator (.roll _returnvalue_2) (.pitch (Math|Rotator|Lerp(Rotator) (Math|Conversions|RotationFromXVector (Transformation|GetActorForwardVector)) (Math|Conversions|RotationFromXVector (Transformation|GetActorUpVector (Variables|Default|GetFlowerTarget))) 0.1)) (.yaw _returnvalue_2)))
    (Transformation|AddActorLocalOffset (Math|Vector|MakeVector (Variables|Default|GetClimbSpeed) 0.0 0.0) false false)
    (if (< (Math|Vector|VectorLength (- (Transformation|GetWorldLocation (Variables|Default|GetMouthLocation)) (Transformation|GetWorldLocation (Variables|/Game/Blueprints/BP_Flower.BP_Flower_C|GetBud (Variables|Default|GetFlowerTarget))))) 2e+01)
      (Utilities|Time|ClearTimerbyFunctionName self "ClimbFlower")
      (CallFunction|ClimbDownFlower))
    (else
      (Variables|Default|SetbClimbing true)
      (Transformation|SetActorRotation (Math|Rotator|FindLookatRotation (Transformation|GetActorLocation) (Transformation|GetWorldLocation (Variables|/Game/Blueprints/BP_Flower.BP_Flower_C|GetBud (Variables|Default|GetFlowerTarget)))))
      (bind _returnvalue_3 (Utilities|Time|SetTimerbyFunctionName _self _returnvalue 0.016 true))
      (Utilities|Time|UnpauseTimerbyHandle _returnvalue_3))))

(fn GetNewFlower
  (bind _outactors (Actor|GetAllActorsOfClass "/Game/Blueprints/BP_Flower.BP_Flower_C"))
  (LocalVariables|SetTempArray _outactors)
  (LocalVariables|SetFlowerCheck (Utilities|Array|Get(acopy) (LocalVariables|GetTempArray) (Math|Random|RandomIntegerinRange 0 (- (Utilities|Array|Length (LocalVariables|GetTempArray)) 1))))
  (while (== (stale _output_get) (Variables|Default|GetFlowerTarget))
    (bind _output_get (LocalVariables|SetFlowerCheck (Utilities|Array|Get(acopy) (LocalVariables|GetTempArray) (Math|Random|RandomIntegerinRange 0 (- (Utilities|Array|Length (LocalVariables|GetTempArray)) 1))))))
  (Variables|Default|SetFlowerTarget (LocalVariables|GetFlowerCheck)))

(fn ClimbDownFlower
  (bind _returnvalue (Utilities|String|MakeLiteralString "ClimbDownFlower"))
  (bind _returnvalue_2 (Transformation|GetActorRotation))
  (bind _returnvalue_3 (Transformation|GetActorLocation))
  (bind _self self)
  (if (Class|KismetSystemLibrary|TimerExists _self _returnvalue)
    (Transformation|AddActorLocalOffset (Math|Vector|MakeVector (Variables|Default|GetClimbSpeed) 0.0 0.0) false false)
    (if (< (Math|Vector|VectorLength (- (Transformation|GetWorldLocation (Variables|Default|GetMouthLocation)) (Transformation|GetActorLocation (Variables|Default|GetFlowerTarget)))) 2e+01)
      (Utilities|Time|ClearTimerbyFunctionName self "ClimbDownFlower")
      (Transformation|SetActorRotation (Math|Rotator|MakeRotator (.roll _returnvalue_2) 0.0 (.yaw _returnvalue_2)))
      (Transformation|SetActorLocation (Math|Vector|MakeVector (.x _returnvalue_3) (.y _returnvalue_3) (+ (.z (Transformation|GetActorLocation (Variables|Default|GetFlowerTarget))) (Variables|/Script/Engine.CapsuleComponent|GetCapsuleHalfHeight (Variables|Collision|GetCapsuleComponent)))) false false)
      (Variables|Default|SetbClimbing false)
      (CallFunction|SearchforFlower))
    (else
      (Transformation|SetActorRotation (Math|Conversions|RotationFromXVector (* (Transformation|GetActorForwardVector) -1.0)))
      (bind _returnvalue_4 (Utilities|Time|SetTimerbyFunctionName _self _returnvalue 0.016 true))
      (Utilities|Time|UnpauseTimerbyHandle _returnvalue_4))))

(fn Wander
  (bind _returnvalue (Transformation|GetActorLocation))
  (bind (_randomlocation _returnvalue_2) (Class|NavigationSystem|GetRandomPointinNavigableRadius _returnvalue 1e+03))
  (while (not _returnvalue_2)
    _)
  (AI|Navigation|SimpleMovetoLocation (AI|GetAIController self) _randomlocation))

(fn OnBeeOverlap
  (bind _self self)
  (Variables|Default|SetbBeeTouching true)
  (AI|Navigation|StopMovement (AI|GetAIController _self))
  (Class|KismetSystemLibrary|PauseTimer _self "Wander")
  (Rendering|SetVisibility (Variables|Default|GetSnailBody) false false)
  (Class|FMODAudioComponent|Play (Variables|Default|GetScream)))

(fn OnBeeEndOverlap
  (bind _returnvalue (Utilities|String|MakeLiteralString "ResumeWander"))
  (bind _self self)
  (Variables|Default|SetbBeeTouching false)
  (if (Class|KismetSystemLibrary|TimerExists _self _returnvalue)
    (if (not (Class|KismetSystemLibrary|IsTimerActive _self _returnvalue))
      (Class|KismetSystemLibrary|UnPauseTimer _self _returnvalue))
    (else
      (bind _returnvalue_2 (Utilities|Time|SetTimerbyFunctionName _self _returnvalue 2.0 true))
      (Utilities|Time|UnpauseTimerbyHandle _returnvalue_2))))

(fn ResumeWander
  (bind _self self)
  (if (not (Variables|Default|GetbBeeTouching))
    (CallFunction|Wander)
    (Class|FMODAudioComponent|Play (Variables|Default|GetBop))
    (Class|KismetSystemLibrary|UnPauseTimer _self "Wander")
    (Utilities|Time|ClearTimerbyFunctionName _self "ResumeWander")
    (Rendering|SetVisibility (Variables|Default|GetSnailBody) true false)))