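; Hanging flower spawner that blooms once, when an actor with "Bee" in its name enters its sphere.
; The overlap reveals the Flowers mesh at a random per-axis scale and tints it with a random colour through a dynamic material instance.
; It then spawns a pollen particle emitter at the sphere and plays Bloom, with a flag blocking repeat triggers.
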(event OnComponentBeginOverlap(Sphere)
  (params (OverlappedComponent :type Primitive%20Component%20Object%20Reference) (OtherActor :type Actor%20Object%20Reference) (OtherComp :type Primitive%20Component%20Object%20Reference) (OtherBodyIndex :type Integer) (bFromSweep :type Boolean) (SweepResult :type Hit%20Result%20Structure%20%28by%20ref%29))
  (bind _returnvalue (Math|Random|RandomFloatinRange 0.7 1.2))
  (bind _sphere (Variables|Default|GetSphere))
  (bind _flowers (Variables|Default|GetFlowers))
  (bind _returnvalue_2 (Transformation|GetWorldTransform _sphere))
  (if (Utilities|String|Contains (Utilities|GetObjectName OtherActor) "Bee")
    (if (not (Variables|Default|GetIsBloomed))
      (Variables|Default|SetIsBloomed true)
      (Rendering|SetVisibility _flowers true false)
      (bind _returnvalue_3 (Rendering|Material|CreateDynamicMaterialInstance _flowers 0 (Rendering|Material|GetMaterial _flowers 0) :!class /Script/Engine.PrimitiveComponent))
      (Transformation|SetRelativeScale3D _flowers (Math|Vector|MakeVector _returnvalue _returnvalue _returnvalue))
      (bind _output_get (Variables|Default|SetFlowerHeadColour (Math|Conversions|ToLinearColor(Vector) (Math|Random|RandomUnitVector))))
      (Rendering|Material|SetVectorParameterValue _returnvalue_3 "BC | Colour Adjustment 2" _output_get :!class /Script/Engine.MaterialInstanceDynamic)
      (Effects|SpawnEmitteratLocation "/Game/Assets/ParticleSystems/pollen_particles.pollen_particles" (.location _returnvalue_2) (.rotation _returnvalue_2) (.scale _returnvalue_2))
      (Class|FMODAudioComponent|Play (Variables|Default|GetBloom)))))

(fn ConstructionScript)