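; BP_Flower is a flower actor that blooms when a bee touches it.
; An overlap on Flower_Head checks whether the other actor's object name contains "Bee".
; If the unbloomed mesh is still visible, it hides it, shows the bloomed one and spawns a pollen particle burst at the FlowerHead transform.
; The visibility check makes the bloom happen only once.
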(event OnComponentBeginOverlap(Flower_Head)
  (params (OverlappedComponent :type Primitive%20Component%20Object%20Reference) (OtherActor :type Actor%20Object%20Reference) (OtherComp :type Primitive%20Component%20Object%20Reference) (OtherBodyIndex :type Integer) (bFromSweep :type Boolean) (SweepResult :type Hit%20Result%20Structure%20%28by%20ref%29))
  (bind _flower_head (Variables|Default|GetFlower_Head))
  (bind _unbloomed (Variables|Default|GetUnBloomed))
  (bind _returnvalue (Transformation|GetWorldTransform _flower_head))
  (if (Utilities|String|Contains (Utilities|GetObjectName OtherActor) "Bee")
    (if (Variables|/Script/Engine.SceneComponent|GetbVisible _unbloomed)
      (Rendering|SetVisibility _unbloomed false false)
      (Rendering|SetVisibility (Variables|Default|GetBloomed) true false)
      (Effects|SpawnEmitteratLocation "/Game/Assets/ParticleSystems/pollen_particles.pollen_particles" (.location _returnvalue) (.rotation _returnvalue) (.scale _returnvalue)))))

(event EventBeginPlay)

(event Collision|EventActorBeginOverlap
  (params (OtherActor :type Actor%20Object%20Reference)))

(event EventTick
  (params (DeltaSeconds :type Float%20%28single-precision%29)))

(fn ConstructionScript)